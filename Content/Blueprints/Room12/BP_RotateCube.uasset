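; BP_RotateCube is an interactable Room 12 actor whose cube the player rotates around yaw with the L and K keys.
; Overlap begin and end toggle the two key prompts, and both call EnableInput, so input is never disabled after leaving.
; Holding L (clockwise) or K (counterclockwise) sets mutually exclusive flags.
; Tick reads them to adjust an accumulated angle by speed times delta time and apply it as relative rotation.
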(event EventBeginPlay)

(event Collision|EventActorBeginOverlap
  (params (OtherActor :type Actor%20Object%20Reference))
  ;[1 1 1] Toggle Text On and Off
  (Utilities|FlowControl|Sequence
    (:then_0
      (Rendering|ToggleVisibility (Variables|Default|GetPress%20L%20Rotate) false))
    (:then_1
      (Rendering|ToggleVisibility (Variables|Default|GetPress%20K%20Rotate) false))
    (:then_2
      ;[1 1 1] Toggle Input On and Off
      (Input|EnableInput (Game|GetPlayerController 0)))))

(event EventTick
  (params (DeltaSeconds :type Float%20%28single-precision%29))
  (bind _cube (Variables|Default|GetCube))
  (bind _speed_of_rotation (Variables|controls|GetSpeed%20of%20Rotation))
  (bind _returnvalue (* _speed_of_rotation DeltaSeconds))
  ;[1 1 1] actor clockwise/counterclockwise
  (Utilities|FlowControl|Sequence
    (:then_0
      (if (Variables|controls|GetRotating%20Clockwise)
        (bind _output_get (Variables|controls|SetCurrent%20Angle%20Deg (+ _returnvalue (Variables|controls|GetCurrent%20Angle%20Deg))))
        (Transformation|SetRelativeRotation _cube (Math|Rotator|MakeRotator 0.0 0.0 _output_get) false false)))
    (:then_1
      (if (Variables|controls|GetRotatingCounterClockwise)
        (bind _output_get_2 (Variables|controls|SetCurrent%20Angle%20Deg (+ (* _returnvalue -1.0) (Variables|controls|GetCurrent%20Angle%20Deg))))
        (Transformation|SetRelativeRotation _cube (Math|Rotator|MakeRotator 0.0 0.0 _output_get_2) false false)))))

(event Collision|EventActorEndOverlap
  (params (OtherActor :type Actor%20Object%20Reference))
  ;[1 1 1] Toggle Text On and Off
  (Utilities|FlowControl|Sequence
    (:then_0
      (Rendering|ToggleVisibility (Variables|Default|GetPress%20L%20Rotate) false))
    (:then_1
      (Rendering|ToggleVisibility (Variables|Default|GetPress%20K%20Rotate) false))
    (:then_2
      ;[1 1 1] Toggle Input On and Off
      (Input|EnableInput (Game|GetPlayerController 0)))))

(event Input|KeyboardEvents|L
  (params (Key :type Key%20Structure :default "None"))
  ;[1 1 1] button pressed boolean
  (:Pressed
    (Variables|controls|SetRotating%20Clockwise true)
    (Variables|controls|SetRotatingCounterClockwise false))
  (:Released
    (Variables|controls|SetRotating%20Clockwise false)))

(event Input|KeyboardEvents|K
  (params (Key :type Key%20Structure :default "None"))
  ;[1 1 1] button pressed boolean
  (:Pressed
    (Variables|controls|SetRotatingCounterClockwise true)
    (Variables|controls|SetRotating%20Clockwise false))
  (:Released
    (Variables|controls|SetRotatingCounterClockwise false)))

(fn ConstructionScript)