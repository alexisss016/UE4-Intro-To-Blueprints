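; BP_LightbulbMulti is a switchable lightbulb prop in Room9 that starts switched off when play begins.
; The construction script creates a dynamic instance of M_Glass on the glass slot of the LightBulb component.
; SwitchLight takes a boolean and sets both the PointLight intensity and the glass material's GlowMultiplier, so the emitted light and visible glow change together.
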(event EventBeginPlay
  (CallFunction|SwitchLight false))

(event Collision|EventActorBeginOverlap
  (params (OtherActor :type Actor%20Object%20Reference)))

(event EventTick
  (params (DeltaSeconds :type Float%20%28single-precision%29)))

(fn ConstructionScript
  (bind _returnvalue (Rendering|Material|CreateDynamicMaterialInstance (Variables|Default|GetLight%20Bulb) 1 "/Game/Materials/M_Glass.M_Glass" "None" :!class /Script/Engine.PrimitiveComponent))
  (Variables|Lightbulb|SetDynamicMaterial _returnvalue))

(fn SwitchLight
  (params (bIsOn :type Boolean))
  (if bIsOn
    ;[1 1 1] Turn Light On
    (Rendering|Components|Light|SetIntensity (Variables|Default|GetPointLight) 5e+03)
    (Rendering|Material|SetScalarParameterValue (Variables|Lightbulb|GetDynamicMaterial) "GlowMultiplier" 5.0 :!class /Script/Engine.MaterialInstanceDynamic)
    (else
      ;[1 1 1] Turn Light On
      (Rendering|Components|Light|SetIntensity (Variables|Default|GetPointLight) 0.0)
      (Rendering|Material|SetScalarParameterValue (Variables|Lightbulb|GetDynamicMaterial) "GlowMultiplier" 0.0 :!class /Script/Engine.MaterialInstanceDynamic))))