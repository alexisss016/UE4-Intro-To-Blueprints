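; Room 8 actor that moves its TranslatingCube component back and forth on any of the X, Y and Z axes.
; Tick accumulates TotalTime and adds its sine as a relative location offset on each axis enabled by the BTranslateOn booleans.
; The per-frame step is not scaled by DeltaSeconds, so travel distance depends on frame rate.
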(event EventBeginPlay)

(event Collision|EventActorBeginOverlap
  (params (OtherActor :type Actor%20Object%20Reference)))

(event EventTick
  (params (DeltaSeconds :type Float%20%28single-precision%29))
  ;[1 1 1] evaluate sin wave
  (bind _output_get (Variables|Default|SetTotal%20Time (+ (Variables|Default|GetTotal%20Time) DeltaSeconds)))
  (Utilities|FlowControl|Sequence
    (:then_0
      ;[1 1 1] translate on z
      (if (Variables|Translation|Get%20bTranslateOnZ)
        (Transformation|AddRelativeLocation (Variables|Default|GetTranslating%20Cube) (Math|Vector|MakeVector 0.0 0.0 (Math|Trig|Sin(Radians) _output_get)) false false)))
    (:then_1
      ;[1 1 1] translate on x
      (if (Variables|Translation|Get%20bTranslateOnX)
        (Transformation|AddRelativeLocation (Variables|Default|GetTranslating%20Cube) (Math|Vector|MakeVector (Math|Trig|Sin(Radians) _output_get) 0.0 0.0) false false)))
    (:then_2
      ;[1 1 1] translate on y
      (if (Variables|Translation|Get%20bTranslateOnY)
        (Transformation|AddRelativeLocation (Variables|Default|GetTranslating%20Cube) (Math|Vector|MakeVector 0.0 (Math|Trig|Sin(Radians) _output_get) 0.0) false false)))))

(fn ConstructionScript)