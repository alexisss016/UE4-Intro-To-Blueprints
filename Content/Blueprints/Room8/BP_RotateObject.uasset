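; BP_RotateObject is an actor that spins continuously at a configurable rate in degrees per second.
; Each Tick scales that rate by delta time for frame-rate independence and applies it on whichever of the X, Y and Z axes are enabled by flags.
; Roll and yaw rotate the RotatingCube component relatively, while pitch applies a local rotation to the whole actor.
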(event EventBeginPlay)

(event Collision|EventActorBeginOverlap
  (params (OtherActor :type Actor%20Object%20Reference)))

(event EventTick
  (params (DeltaSeconds :type Float%20%28single-precision%29))
  (Variables|Default|SetDegrees%20Since%20Last%20Frame (* DeltaSeconds (Variables|Default|GetDegrees%20Per%20Second)))
  (Utilities|FlowControl|Sequence
    (:then_0
      ;[1 1 1] Adjust Yaw
      (if (Variables|rotate|GetbRotateOnZ)
        (Transformation|AddRelativeRotation (Variables|Default|GetRotating%20Cube) (Math|Rotator|MakeRotator 0.0 0.0 (Variables|Default|GetDegrees%20Since%20Last%20Frame)) false false)))
    (:then_1
      ;[1 1 1] Adjust Pitch
      (if (Variables|rotate|GetbRotateOnY)
        (Transformation|AddActorLocalRotation (Math|Rotator|MakeRotator 0.0 (Variables|Default|GetDegrees%20Since%20Last%20Frame) 0.0) false false)))
    (:then_2
      ;[1 1 1] Adjust Roll
      (if (Variables|rotate|GetbRotateOnX)
        (Transformation|AddRelativeRotation (Variables|Default|GetRotating%20Cube) (Math|Rotator|MakeRotator (Variables|Default|GetDegrees%20Since%20Last%20Frame) 0.0 0.0) false false)))))

(fn ConstructionScript)