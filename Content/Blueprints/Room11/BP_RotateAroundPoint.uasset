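; BP_RotateAroundPoint is an actor that orbits a target actor at a set radius, speed and direction.
; Tick accumulates a wrapped angle, then rotates the target's scaled right vector around its up vector to position the actor, adding a starting offset.
; It turns to face the target only when debug radius drawing is enabled, alongside the debug line.
; On-screen prints show the optional angle readout and flag a missing target.
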(event EventBeginPlay)

(event Collision|EventActorBeginOverlap
  (params (OtherActor :type Actor%20Object%20Reference)))

(event EventTick
  (params (DeltaSeconds :type Float%20%28single-precision%29))
  (bind _target_to_rotate_around (Variables|Targets|GetTarget%20To%20Rotate%20Around))
  (Utilities|FlowControl|Sequence
    (:then_0
      ;[1 1 1] Set Current Rotation in Degrees
      (bind _output_get (Variables|Rotation|SetCurrent%20Angle%20In%20Degrees (Math|Float|%(Float) (+ (Variables|Rotation|GetCurrent%20Angle%20In%20Degrees) (* (Variables|Rotation|GetDegrees%20Per%20Second) DeltaSeconds (Math|Float|SelectFloat 1.0 -1.0 (Variables|Rotation|GetClockwise)))) 359.0)))
      (Development|PrintString (Utilities|String|ToString(Float) _output_get) (Variables|debug|GetShow%20Debug%20Angle%20In%20Degrees) true "(R=0.000000,G=0.660000,B=1.000000,A=1.000000)" 0.0))
    (:then_1
      ;[1 1 1] rotate around target
      (Utilities|IsValid _target_to_rotate_around
        (:Is%20Valid
          ;;[1 1 1] repposition actor in new position
          (Transformation|SetActorLocation (+ (Transformation|GetActorLocation (Variables|Targets|GetTarget%20To%20Rotate%20Around)) (Math|Vector|RotateVectorAroundAxis (* (Transformation|GetActorRightVector (Variables|Targets|GetTarget%20To%20Rotate%20Around)) (Variables|Rotation|Getradius)) (+ (Variables|Rotation|GetCurrent%20Angle%20In%20Degrees) (Variables|Rotation|GetStarting%20Angle)) (Transformation|GetActorUpVector _target_to_rotate_around))) false false)
          (if (Variables|debug|Get%20Draw%20Debug%20Radius)
            (Rendering|Debug|DrawDebugLine :LineStart (+ (Transformation|GetActorLocation (Variables|Targets|GetTarget%20To%20Rotate%20Around)) (Math|Vector|RotateVectorAroundAxis (* (Transformation|GetActorRightVector (Variables|Targets|GetTarget%20To%20Rotate%20Around)) (Variables|Rotation|Getradius)) (+ (Variables|Rotation|GetCurrent%20Angle%20In%20Degrees) (Variables|Rotation|GetStarting%20Angle)) (Transformation|GetActorUpVector _target_to_rotate_around))) :LineEnd (Transformation|GetActorLocation (Variables|Targets|GetTarget%20To%20Rotate%20Around)) :Thickness 3.0)
            ;[1 1 1] make actor look like at target
            (Transformation|SetActorRotation (Math|Rotator|FindLookatRotation (Transformation|GetActorLocation) (Transformation|GetActorLocation (Variables|Targets|GetTarget%20To%20Rotate%20Around))))))
        (:Is%20Not%20Valid
          ;;[1 1 1] error, dont want to see
          (Development|PrintString "no object to rotate around" true true "(R=0.163079,G=0.000000,B=1.000000,A=1.000000)" 0.0))))))

(fn ConstructionScript)