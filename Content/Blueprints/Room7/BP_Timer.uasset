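; BP_Timer is a Room 7 timer that shows elapsed time on two text components, MSTimer and SecTimer.
; Each Tick adds DeltaSeconds to TimeInMilliseconds, which therefore holds fractional seconds despite its name, and writes it to MSTimer.
; A second Tick branch uses a one-second Delay, which ignores calls while pending, to increment the whole-second count about once per second and update SecTimer.
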(event EventBeginPlay)

(event Collision|EventActorBeginOverlap
  (params (OtherActor :type Actor%20Object%20Reference))
  ;[1 1 1] Render time to set MS Timer text component
)

(event EventTick
  (params (DeltaSeconds :type Float%20%28single-precision%29))
  (Utilities|FlowControl|Sequence
    (:then_0
      ;[1 1 1] Update Time in Miliseconds
      (bind _output_get (Variables|TImer|SetTime%20in%20Milliseconds (+ (Variables|TImer|GetTime%20in%20Milliseconds) DeltaSeconds)))
      ;[1 1 1] Render time to set MS Timer text component
      (Rendering|Components|TextRender|SetText (Variables|Default|GetMS%20Timer) (Utilities|Text|ToText(Float) _output_get "HalfToEven")))
    (:then_1
      ;[1 1 1] Update time in seconds
      (Utilities|FlowControl|Delay 1.0)
      (bind _output_get_2 (Variables|Timer|SetTime%20in%20Seconds (+ (Variables|Timer|GetTime%20in%20Seconds) 1)))
      ;[1 1 1] Render Time in seconds to sec timer text component
      (Rendering|Components|TextRender|SetText (Variables|Default|GetSec%20Timer) (Utilities|Text|ToText(Integer) _output_get_2)))))

(fn ConstructionScript)